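; BP_Enemy is an enemy that turns to face and attacks the player character when its PawnSensing component sees it.
; Each sighting rotates the actor toward BP_ThirdPersonCharacter, then, if CanAttack is set, spawns a BP_EnemyProjectile at SpawnProjectileLocation.
; Damage is applied directly to the character at the moment of firing rather than on projectile impact in this graph.
; A short Delay resets CanAttack to limit the fire rate.
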(event `self.PawnSensing.OnSeePawn`
  (params (Pawn :type "Pawn Object Reference"))
  (bind _asbp_third_person_character (cast `/Game/ThirdPerson/Blueprints/BP_ThirdPersonCharacter` Pawn))
  (`self.K2_SetActorRotation` (`KismetMathLibrary.FindRelativeLookAtRotation` (`KismetMathLibrary.Conv_VectorToTransform` (`self.K2_GetActorLocation`)) (`self.K2_GetActorLocation` _asbp_third_person_character)))
  (if (`self.CanAttack`)
    (`|SpawnActorFromClass` "/Game/Blueprints/BP_EnemyProjectile.BP_EnemyProjectile_C" (`SceneComponent.K2_GetComponentToWorld` (`self.SpawnProjectileLocation`)) "Undefined" "MultiplyWithRoot" null null)
    (`GameplayStatics.ApplyDamage` _asbp_third_person_character 10.0)
    (set `self.CanAttack` false)
    (`KismetSystemLibrary.Delay` 0.5)
    (set `self.CanAttack` true)))

(fn `UserConstructionScript`)