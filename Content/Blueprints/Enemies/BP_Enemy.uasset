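; BP_Enemy is an enemy that turns to face and shoots at the third-person player character when its PawnSensing component sees it.
; While CanAttack is true, it spawns a BP_EnemyProjectile, then after a short delay stops the projectile's physics and damages the player directly, without a hit check.
; CanAttack is cleared only after that delay, then restored following a brief cooldown.
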(event `self.PawnSensing.OnSeePawn`
  (params (Pawn :type "Pawn Object Reference"))
  (bind _asbp_third_person_character (cast `/Game/ThirdPerson/Blueprints/BP_ThirdPersonCharacter` Pawn))
  (`self.K2_SetActorRotation` (`KismetMathLibrary.FindRelativeLookAtRotation` (`KismetMathLibrary.Conv_VectorToTransform` (`self.K2_GetActorLocation`)) (`self.K2_GetActorLocation` _asbp_third_person_character)))
  (if (`self.CanAttack`)
    (bind _returnvalue (`|SpawnActorFromClass` "/Game/Blueprints/Enemies/BP_EnemyProjectile.BP_EnemyProjectile_C" (`SceneComponent.K2_GetComponentToWorld` (`self.SpawnProjectileLocation`)) "Undefined" "MultiplyWithRoot" null null))
    (`KismetSystemLibrary.Delay` 0.2)
    (`PrimitiveComponent.SetSimulatePhysics` (`/Game/Blueprints/Enemies/BP_EnemyProjectile.Sphere` _returnvalue) false)
    (`GameplayStatics.ApplyDamage` _asbp_third_person_character 10.0)
    (set `self.CanAttack` false)
    (`KismetSystemLibrary.Delay` 0.5)
    (set `self.CanAttack` true)))

(fn `UserConstructionScript`)